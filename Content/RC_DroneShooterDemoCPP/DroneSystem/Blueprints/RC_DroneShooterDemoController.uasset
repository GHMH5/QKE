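; Player controller for the drone shooter demo that forwards shoot input and tracks the player's score.
; On BeginPlay it creates the Score widget, adds it to the viewport, zeroes the display and sends a game-start message to the game mode.
; Shoot presses are relayed to the controlled pawn as a message.
; Score update events add to the running total and refresh the widget, and a getter exposes the total.
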(event EventBeginPlay
  (CallFunction|CreateScore)
  (CallFunction|UpdateScore)
  (Class|GameModeBPI|HandleGameStart(Message) (Game|GetGameMode)))

(event EventTick
  (params (DeltaSeconds :type Float%20%28single-precision%29)))

(event EventHandleUpdateScore
  (params (Value :type Integer))
  (CallFunction|UpdateScore Value))

(event Input|ActionEvents|InputActionShoot
  (params (Key :type Key%20Structure))
  (:Pressed
    (Class|DroneBPI|HandleShoot(Message) (Pawn|GetControlledPawn))))

(fn ConstructionScript)

(fn UpdateScore
  (params (Score%20To%20Add :type Integer))
  (bind _output_get (Variables|Default|SetPlayerScore (+ Score%20To%20Add (Variables|Default|GetPlayerScore))))
  (Default|UpdateScoreDisplay (Variables|Default|GetScoreWidget) _output_get))

(fn CreateScore
  (bind _returnvalue (UserInterface|CreateWidget "/Game/RC_DroneShooterDemoCPP/DroneSystem/UMG/Score.Score_C"))
  (bind _output_get (Variables|Default|SetScoreWidget _returnvalue))
  (UserInterface|Viewport|AddtoViewport _output_get 0)
  (return))

(fn GetScore
  (return (Variables|Default|GetPlayerScore)))