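; Game mode Blueprint for the drone shooter demo that tracks remaining targets and ends the game when none are left.
; AddTarget and RemoveTarget events adjust the target count, and a removal that brings it to zero calls HandleGameOver.
; HandleGameOver shows the game over widget and switches to UI-only input with a visible cursor.
; HandleGameStart restores game-only input and hides the cursor.
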(event EventAddTarget
  (Variables|Default|SetTargets%20Remaining (+ (Variables|Default|GetTargets%20Remaining) 1)))

(event EventRemoveTarget
  (Variables|Default|SetTargets%20Remaining (- (Variables|Default|GetTargets%20Remaining) 1))
  (if (<= (Variables|Default|GetTargets%20Remaining) 0)
    (CallFunction|HandleGameOver)))

(event EventHandleGameStart
  (bind _returnvalue (Game|GetPlayerController 0))
  (Input|SetInputModeGameOnly _returnvalue)
  (Variables|/Script/Engine.PlayerController|SetbShowMouseCursor _returnvalue false))

(fn ConstructionScript)

(fn HandleGameOver
  (bind _returnvalue (Game|GetPlayerController 0))
  (bind _returnvalue_2 (UserInterface|CreateWidget "/Game/RC_DroneShooterDemoCPP/DroneSystem/UMG/GameOverScreen.GameOverScreen_C"))
  (bind _output_get (Variables|Default|SetGameOverScreen%20Widget _returnvalue_2))
  (UserInterface|Viewport|AddtoViewport _output_get 0)
  (Input|SetInputModeUIOnly _returnvalue 0 "DoNotLock")
  (Variables|/Script/Engine.PlayerController|SetbShowMouseCursor _returnvalue true)
  (return))