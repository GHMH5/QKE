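; Shootable target actor for a drone shooter that awards points when hit and tracks its own health.
; On BeginPlay it creates a dynamic material for its cube and registers with the game mode.
; Each hit scores for the hitter, lowers health and updates the color, which snaps from green to red because the health ratio is truncated.
; At zero health it awards a bonus, unregisters from the game mode and destroys itself.
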(event EventBeginPlay
  (bind _output_get (Variables|Default|SetStartingHealthValue (Variables|Default|GetHealthValue)))
  (bind _returnvalue (Rendering|Material|CreateDynamicMaterialInstance (Variables|Default|GetCube) _output_get "/Game/RC_DroneShooterDemoCPP/SpecialMaterials/TargetMat.TargetMat" :!class /Script/Engine.PrimitiveComponent))
  (Variables|Default|SetDynamicMat _returnvalue)
  (Rendering|Material|SetMaterial (Variables|Default|GetCube) 0 (Variables|Default|GetDynamicMat))
  (CallFunction|SetColor)
  (Class|GameModeBPI|AddTarget(Message) (Game|GetGameMode)))

(event EventHandleWasHit
  (params (Hitter :type Actor%20Object%20Reference) (DamageValue :type Integer))
  (Variables|Default|SetHitter Hitter)
  (Variables|Default|SetDamage%20Value DamageValue)
  (Class|ControllerBPI|HandleUpdateScore(Message) (Variables|Default|GetHitter) (Variables|Default|GetTarget%20Value))
  (Variables|Default|SetHealthValue (- (Variables|Default|GetHealthValue) (Variables|Default|GetDamage%20Value)))
  (CallFunction|SetColor)
  (if (<= (Variables|Default|GetHealthValue) 0)
    (Class|ControllerBPI|HandleUpdateScore(Message) (Variables|Default|GetHitter) (Variables|Default|GetBonusValue))
    (Class|GameModeBPI|RemoveTarget(Message) (Game|GetGameMode))
    (Actor|DestroyActor)))

(fn ConstructionScript)

(fn SetColor
  (Rendering|Material|SetVectorParameterValue (Variables|Default|GetDynamicMat) "Color" (Math|Color|Lerp(LinearColor) "(R=1.000000,G=0.000000,B=0.000000,A=1.000000)" "(R=0.000000,G=1.000000,B=0.000000,A=1.000000)" (Math|Conversions|ToFloat(Integer) (Math|Float|Truncate (/ (Math|Conversions|ToFloat(Integer) (Variables|Default|GetHealthValue)) (Math|Conversions|ToFloat(Integer) (Variables|Default|GetStartingHealthValue)))))) :!class /Script/Engine.MaterialInstanceDynamic)
  (return))